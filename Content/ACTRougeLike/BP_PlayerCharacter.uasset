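; BP_PlayerCharacter is the player character Blueprint for the ACTRougeLike game.
; On BeginPlay it registers the sprint and projectile attack actions with its ActionComp.
; It reads Health from AttributeComp and prints it on screen every tick as debug output, and also prints the new value whenever OnHealthChanged fires.
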(event OnHealthChanged(AttributeComp)
  (params (InstigatorActor :type Actor%20Object%20Reference) (OwningComp :type S%20Attribute%20Component%20Object%20Reference) (NewHealth :type Float%20%28single-precision%29) (Delta :type Float%20%28single-precision%29))
  (Development|PrintString (Utilities|String|ToString(Float) NewHealth)))

(event EventBeginPlay
  (bind _actioncomp (Variables|Default|GetActionComp))
  (Class|SActionComponent|AddAction _actioncomp "/Game/ACTRougeLike/Actions/BP_Sprint.BP_Sprint_C")
  (Class|SActionComponent|AddAction _actioncomp "/Game/ACTRougeLike/Actions/BP_ProjectileAttack.BP_ProjectileAttack_C"))

(event EventTick
  (params (DeltaSeconds :type Float%20%28single-precision%29))
  (Development|PrintString (Class|KismetStringLibrary|BuildStringDouble "" "Health: " (Variables|/Script/ACTRougeLike.SAttributeComponent|GetHealth (Variables|Default|GetAttributeComp))) true false "(R=1.000000,G=0.000000,B=0.014042,A=1.000000)" 0.0))

(fn ConstructionScript)