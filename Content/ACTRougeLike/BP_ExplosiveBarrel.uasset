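; BP_ExplosiveBarrel is an actor for a barrel that explodes on a fixed timer after it spawns.
; On BeginPlay only the authority starts the timer, which calls Explode to run MulticastExplode and set a short lifespan for delayed removal.
; MulticastExplode prints a debug message, fires the radial force impulse, hides the actor and disables its collision.
; A DestroyActor node is left unconnected.
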(event Custom|Explode
  (CallFunction|MulticastExplode)
  (Actor|SetLifeSpan 2.0))

(event Custom|MulticastExplode
  (Development|PrintString "EXPLODE!" true true "(R=1.000000,G=0.405876,B=0.000000,A=1.000000)" 1e+01)
  (Class|RadialForceComponent|FireImpulse (Variables|Default|GetRadialForce1))
  (Rendering|SetActorHiddenInGame true)
  (Collision|SetActorEnableCollision false))

(event EventBeginPlay
  (if (Ability|HasAuthority)
    (Utilities|Time|SetTimerbyEvent (delegate Custom|Explode) 4.0)))

(fn ConstructionScript)